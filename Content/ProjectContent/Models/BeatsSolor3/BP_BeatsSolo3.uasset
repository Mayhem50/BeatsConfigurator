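; Actor for a Beats Solo3 model that plays a folding animation on its two sides, apparently the headphone earcups.
; After a short delay on BeginPlay, the RightCollapse timeline pitches RSphere, then LeftCollapse pitches LSphere once it finishes.
; The right side uses its track as the Lerp alpha, while the left feeds its track into A with a constant alpha above one, extrapolating the angle.
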(event `self.ReceiveBeginPlay`
  (`KismetSystemLibrary.Delay` 0.2)
  (bind (_direction _angle) (`Timeline|RightCollapse`)
    (:`Update`
      (`SceneComponent.K2_SetRelativeRotation` (`self.R_Sphere`) (`KismetMathLibrary.MakeRotator` 0.0 (`KismetMathLibrary.Lerp` 0.0 77.300003 _angle)) false false))
    (:`Finished`
      (bind (_direction_2 _driver) (`Timeline|LeftCollapse`)
        (:`Update`
          (`SceneComponent.K2_SetRelativeRotation` (`self.L_Sphere`) (`KismetMathLibrary.MakeRotator` 0.0 (`KismetMathLibrary.Lerp` _driver 0.0 46.189999)) false false))))))

(fn `UserConstructionScript`)